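; Turret actor that rotates to face enemies entering its overlap area; it has no firing logic.
; Overlap begin matches actor tags against TargetEnemiesTags and stores a transform snapshot, not an actor reference.
; Overlap end removes by the actor's current transform, so moved actors may stay listed.
; Tick aims at the first stored transform, but only when the array length is at most one, including empty.
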(event `self.ReceiveTick`
  (params (DeltaSeconds :type "Float (single-precision)"))
  (`self.LookAtEnemy`))

(event `OnActorBeginOverlap_Event`
  (params (OverlappedActor :type "Actor Object Reference") (OtherActor :type "Actor Object Reference"))
  (`self.CheckAndAddNewTarget` OtherActor))

(event `OnActorEndOverlap_Event`
  (params (OverlappedActor :type "Actor Object Reference") (OtherActor :type "Actor Object Reference"))
  (`KismetArrayLibrary.Array_RemoveItem` (`self.ArrayDetectionsTransforms`) (`self.GetTransform` OtherActor)))

(fn `CheckAndAddNewTarget`
  (params (DetectionActor :type "Actor Object Reference"))
  (bind _isenemy (`self.IsTargetEnemy` (`Actor.Tags` DetectionActor) (`self.TargetEnemiesTags`)))
  (if _isenemy
    (`KismetArrayLibrary.Array_AddUnique` (`self.ArrayDetectionsTransforms`) (`self.GetTransform` DetectionActor))))

(fn `IsTargetEnemy`
  (params (EntityDetectionTags :type "Array of Name") (TargetEnemiesTags :type "Array of Name"))
  (returns (IsEnemy :type Boolean))
  (for _array_element EntityDetectionTags
    (for _array_element_2 TargetEnemiesTags
      (bind _returnvalue (== _array_element_2 _array_element))
      (if _returnvalue
        (break)))
    (if _returnvalue
      (break)))
  (return _returnvalue))

(fn `LookAtEnemy`
  (bind _arraydetectionstransforms (`self.ArrayDetectionsTransforms`))
  (if (>= 1 (`KismetArrayLibrary.Array_Length` _arraydetectionstransforms))
    (`self.K2_SetActorTransform` (`KismetAnimationLibrary.K2_LookAt` (`self.GetTransform`) (`KismetMathLibrary.TransformLocation` (`|GetArrayItem` _arraydetectionstransforms))))))

(fn `UserConstructionScript`)